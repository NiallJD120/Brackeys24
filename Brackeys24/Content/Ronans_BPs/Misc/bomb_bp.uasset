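; Countdown bomb actor that damages the player if they are inside its Box when time runs out.
; Tick decrements a clamped Time value and shows it as whole seconds on a TextRender.
; At zero, an overlapping player takes damage with a Niagara fireball and a short delay before the bomb is destroyed; otherwise it is destroyed without an explosion.
; The timer re-set every Tick targets an empty event, so Tick alone drives detonation.
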(event `self.ReceiveTick`
  (params (DeltaSeconds :type "Float (single-precision)"))
  (bind _time (`self.Time`))
  (bind _returnvalue (`KismetMathLibrary.FClamp` (- _time DeltaSeconds) 0.0 _time))
  (`KismetSystemLibrary.K2_SetTimerDelegate` (delegate `BoomBoomBOom`) _time)
  (bind _output_get (set `self.Time` _returnvalue))
  (`TextRenderComponent.K2_SetText` (`self.TextRender`) (`KismetTextLibrary.Conv_IntToText` (`KismetMathLibrary.FTrunc` _returnvalue)))
  (bind _asplayer_character_bp (cast `/Game/Ronans_BPs/Character/PlayerCharacter_BP` (`GameplayStatics.GetPlayerCharacter` 0)))
  ;[1 1 1] Add scene component here
  (if (== _output_get 0.0)
    (if (`PrimitiveComponent.IsOverlappingActor` (`self.Box`) _asplayer_character_bp)
      (`NiagaraFunctionLibrary.SpawnSystemAtLocation` "/Game/Nialls-BPs/Particles/FireballExplode1.FireballExplode1" (`self.K2_GetActorLocation`))
      (`GameplayStatics.ApplyDamage` _asplayer_character_bp 20.0 null null "/Script/Engine.DamageType")
      (`KismetSystemLibrary.Delay` 0.2)
      (`KismetSystemLibrary.PrintString` "rh2jhnfiw"))
    (`self.K2_DestroyActor`)))

(event `BoomBoomBOom`)

(fn `UserConstructionScript`)